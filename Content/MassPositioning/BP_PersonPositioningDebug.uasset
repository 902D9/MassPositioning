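; BP_PersonPositioningDebug is a debug Blueprint that feeds generated test data into the Mass-based personnel positioning simulation.
; A looping one-second timer generates debug positioning points and person data, seeded by the previous batch.
; The first batch starts the PersonnelPositioningSubsystem simulation with the agent config.
; Once stored points exist, later batches update that simulation instead, and each batch is cached for the next tick.
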(event Custom|Debug
  (bind _returnvalue (Subsystems|GetPersonnelPositioningSubsystem))
  (bind (_debugpositioningpoints _debugpersondata _generatedpoints) (Class|PositioningDebugLibrary|GeneratePositioningDebugPoints (Variables|Default|GetGenerated%20Points) 99))
  (Utilities|FlowControl|Sequence
    (:then_0
      (if (Utilities|Array|IsValidIndex (Variables|Default|GetGenerated%20Points))
        (Class|PersonnelPositioningSubsystem|UpdatePersonnelPositioningSimulation _returnvalue _debugpositioningpoints _debugpersondata)
        (else
          (Class|PersonnelPositioningSubsystem|StartPersonnelPositioningSimulation _returnvalue _debugpositioningpoints _debugpersondata "/Game/MassPositioning/AI/MassPersonnelPositioningAgentConfig.MassPersonnelPositioningAgentConfig"))))
    (:then_1
      (Variables|Default|SetGenerated%20Points _generatedpoints))))

(event EventBeginPlay
  (Utilities|Time|SetTimerbyEvent (delegate Custom|Debug) 1.0 true))

(fn ConstructionScript)